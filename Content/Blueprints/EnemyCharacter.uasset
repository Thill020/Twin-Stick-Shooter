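; Enemy character for a twin-stick shooter that deals repeated damage to the hero while overlapping.
; A looping timer, set by attack rate, starts on hero overlap and clears when it ends.
; On death it drops collision responses, adds score through TwinStickMode, detaches its controller, then after a delay occasionally spawns a bullet upgrade pickup and destroys itself.
; The construction script tints its body through a dynamic material.
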(event `SpawnProjectileUpgrade`
  ;[1 1 1] Spawn projectile 1/10th of the time of death
  (if (> (`KismetMathLibrary.RandomInteger` 21) 18)
    (`|SpawnActorFromClass` "/Game/Blueprints/BulletPickupUpgrade.BulletPickupUpgrade_C" (`self.GetTransform` self) "Undefined" "OverrideRootScale" null null)))

(event `/Game/Blueprints/iDamageable.AffectHealth`
  (params (Delta :type "Float (single-precision)"))
  (bind _capsulecomponent (`self.CapsuleComponent`))
  ;[1 1 1] Determine When to Damage Player
  (`self.CalculateHealth` Delta)
  (if (`self.isDead`)
    (`PrimitiveComponent.SetCollisionResponseToChannel` _capsulecomponent "ECC_WorldDynamic" "ECR_Ignore")
    (`PrimitiveComponent.SetCollisionResponseToChannel` _capsulecomponent "ECC_Pawn" "ECR_Ignore")
    (bind _astwin_stick_mode (cast `/Game/Blueprints/TwinStickMode` (`GameplayStatics.GetGameMode`)))
    (`/Game/Blueprints/TwinStickMode.IncrementScore` _astwin_stick_mode (`self.Delta Score`))
    (`self.DetachFromControllerPendingDestroy`)
    (`KismetSystemLibrary.Delay` 3.0)
    (`self.SpawnProjectileUpgrade`)
    (`self.K2_DestroyActor`)))

(event `self.ReceiveActorBeginOverlap`
  (params (OtherActor :type "Actor Object Reference"))
  ;[1 1 1] Start Damaging the Player on Overlap
  (bind _ashero_character (cast `/Game/Blueprints/HeroCharacter` OtherActor))
  (set `self.Hero` _ashero_character)
  (`KismetSystemLibrary.K2_SetTimer` null "DamageTheHero" (/ 1.0 (`self.AttacksPerSecond`)) true))

(event `DamageTheHero`
  ;[1 1 1] Damage Player
  (`/Game/Blueprints/HeroCharacter.AffectHealth` (`self.Hero`) (`self.Delta`)))

(event `self.ReceiveActorEndOverlap`
  (params (OtherActor :type "Actor Object Reference"))
  ;[1 1 1] Stop Damaging Player
  (if (== OtherActor (`self.Hero`))
    (`KismetSystemLibrary.K2_ClearTimer` null "DamageTheHero")))

(fn `UserConstructionScript`
  (bind _returnvalue (`PrimitiveComponent.CreateDynamicMaterialInstance` (`self.Mesh`) 0 null "None"))
  (bind _output_get (set `self.Dyna Mat` _returnvalue))
  (`MaterialInstanceDynamic.SetVectorParameterValue` _output_get "BodyColor" (`self.Enemy Color`)))