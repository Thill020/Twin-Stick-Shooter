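; Enemy spawner for a twin-stick game that adds normal, fast and strong AI enemies at random points inside its SpawnVolume.
; Each SpawnEnemy call counts live actors of the three classes against MaxEnemies, which IncreaseSpawnLimit raises.
; Below the limit, the cached TwinStickMode's Phase picks a random mix, shifting from only normal enemies to fast and strong ones.
; EnemyCount is tallied separately and not used by the limit check.
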(event `self.ReceiveBeginPlay`
  ;[1 1 1] Cashe the GameMode
  (bind _astwin_stick_mode (cast `/Game/Blueprints/TwinStickMode` (`GameplayStatics.GetGameMode`)))
  (set `self.Twin Stick Mode` _astwin_stick_mode))

(event `IncreaseSpawnLimit`
  (params (`Add To Spawn Limit` :type Integer))
  ;[1 1 1] Add Number to Spawn Limit
  (set `self.MaxEnemies` (+ `Add To Spawn Limit` (`self.MaxEnemies`))))

(event `AddToEnemyCount`
  (params (Count :type Integer))
  ;[1 1 1] Event to add Fast and Strong enemies to enemy count
  (set `self.EnemyCount` (+ Count (`self.EnemyCount`))))

(event `SpawnEnemy`
  (bind _returnvalue (`KismetMathLibrary.RandomInteger` 3))
  ;[1 1 1] If there are less enemies than the max allowed number of Enemies, Spawn more abased on Phase
  ;;[1 1 1] Combine the number of all possible enemies
  (bind _outactors (`GameplayStatics.GetAllActorsOfClass` "/Game/Blueprints/EnemyCharacter.EnemyCharacter_C"))
  (bind _outactors_2 (`GameplayStatics.GetAllActorsOfClass` "/Game/Blueprints/EnemyCharacter_Fast.EnemyCharacter_Fast_C"))
  (bind _outactors_3 (`GameplayStatics.GetAllActorsOfClass` "/Game/Blueprints/EnemyCharacter_Strong.EnemyCharacter_Strong_C"))
  (if (< (+ (`KismetArrayLibrary.Array_Length` _outactors_3) (`KismetArrayLibrary.Array_Length` _outactors_2) (`KismetArrayLibrary.Array_Length` _outactors)) (`self.MaxEnemies`))
    ;;[1 1 1] Phase 1
    (if (== (`/Game/Blueprints/TwinStickMode.Phase` (`self.Twin Stick Mode`)) 1)
      (`self.SpawnNormalEnemy`)
      (else
        ;;[1 1 1] Phase 2
        (if (== (`/Game/Blueprints/TwinStickMode.Phase` (`self.Twin Stick Mode`)) 2)
          (if (== (`KismetMathLibrary.RandomInteger` 3) 2)
            (`self.SpawnFastEnemy`)
            (else
              (`self.SpawnNormalEnemy`)))
          (else
            ;;[1 1 1] Phase 3
            (if (== (`/Game/Blueprints/TwinStickMode.Phase` (`self.Twin Stick Mode`)) 3)
              (if (== _returnvalue 2)
                (`self.SpawnFastEnemy`)
                (elif (== _returnvalue 1)
                  (`self.SpawnNormalEnemy`)
                  (else
                    (`self.SpawnStrongEnemy`))))
              (else
                ;;[1 1 1] Phase 4
                (if (== (`/Game/Blueprints/TwinStickMode.Phase` (`self.Twin Stick Mode`)) 4)
                  (if (== (`KismetMathLibrary.RandomInteger` 3) 2)
                    (`self.SpawnStrongEnemy`)
                    (else
                      (`self.SpawnFastEnemy`)))
                  (else
                    ;;[1 1 1] Phase 5
                    (if (== (`KismetMathLibrary.RandomInteger` 2) 1)
                      (`self.SpawnStrongEnemy`)
                      (else
                        (`self.SpawnFastEnemy`)))))))))))))

(event `SpawnNormalEnemy`
  (bind _spawnvolume (`self.SpawnVolume`))
  ;[1 1 1] Spawn Functions
  ;;[1 1 1] Spawn Normal Enemy
  (`AIBlueprintHelperLibrary.SpawnAIFromClass` "/Game/Blueprints/EnemyCharacter.EnemyCharacter_C" null (`KismetMathLibrary.RandomPointInBoundingBox` (`SceneComponent.K2_GetComponentLocation` _spawnvolume) (`BoxComponent.GetScaledBoxExtent` _spawnvolume)) (struct) false null))

(event `SpawnFastEnemy`
  (bind _spawnvolume (`self.SpawnVolume`))
  ;[1 1 1] Spawn Functions
  ;;[1 1 1] Spawn Fast Enemy
  (`AIBlueprintHelperLibrary.SpawnAIFromClass` "/Game/Blueprints/EnemyCharacter_Fast.EnemyCharacter_Fast_C" null (`KismetMathLibrary.RandomPointInBoundingBox` (`SceneComponent.K2_GetComponentLocation` _spawnvolume) (`BoxComponent.GetScaledBoxExtent` _spawnvolume)) (struct) false null))

(event `SpawnStrongEnemy`
  (bind _spawnvolume (`self.SpawnVolume`))
  ;[1 1 1] Spawn Functions
  ;;[1 1 1] Spawn Strong Enemy
  (`AIBlueprintHelperLibrary.SpawnAIFromClass` "/Game/Blueprints/EnemyCharacter_Strong.EnemyCharacter_Strong_C" null (`KismetMathLibrary.RandomPointInBoundingBox` (`SceneComponent.K2_GetComponentLocation` _spawnvolume) (`BoxComponent.GetScaledBoxExtent` _spawnvolume)) (struct) false null))

(fn `UserConstructionScript`)