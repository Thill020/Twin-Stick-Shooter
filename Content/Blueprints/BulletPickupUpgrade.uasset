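; BulletPickupUpgrade is a pickup that temporarily switches the overlapping HeroCharacter's weapon to twin fire.
; On overlap it teleports itself aside, sets the weapon's ProjectileFunction by name to "FireTwin" and releases the trigger.
; After UpgradeDuration it restores "Fire", releases the trigger again and destroys itself.
; On BeginPlay it destroys itself if another instance exists, including one still timing an active upgrade.
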(event `self.ReceiveActorBeginOverlap`
  (params (OtherActor :type "Actor Object Reference"))
  ;[1 1 1] When player overlaps the upgrade, apply the upgrade, and then destroy it once the duration expires
  (bind _ashero_character (cast `/Game/Blueprints/HeroCharacter` OtherActor))
  (`self.K2_SetActorLocation` (-100.0 -100.0 -100.0) false true)
  (bind _weapon (`/Game/Blueprints/HeroCharacter.Weapon` _ashero_character))
  (set `/Game/Blueprints/Weapon.ProjectileFunction` "FireTwin" _weapon)
  (`/Game/Blueprints/Weapon.ReleaseTrigger` _weapon)
  (`KismetSystemLibrary.Delay` (`self.UpgradeDuration`))
  (set `/Game/Blueprints/Weapon.ProjectileFunction` "Fire" _weapon)
  (`/Game/Blueprints/Weapon.ReleaseTrigger` _weapon)
  (`self.K2_DestroyActor`))

(event `self.ReceiveBeginPlay`
  ;[1 1 1] Ensure that only one upgrade node is in play at a time, if another spawns, destroy it.
  (bind _outactors (`GameplayStatics.GetAllActorsOfClass` "BulletPickupUpgrade_C"))
  (if (> (`KismetArrayLibrary.Array_Length` _outactors) 1)
    (`self.K2_DestroyActor`)))

(fn `UserConstructionScript`)