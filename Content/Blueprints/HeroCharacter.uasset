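; HeroCharacter is the twin-stick player character, with axis-driven world-space movement, aiming and firing.
; On BeginPlay it attaches a spawned weapon to GunSocket, records its spawn transform in TwinStickMode and creates the HUD.
; Look input past a deadzone sets control rotation and pulls the weapon's trigger, otherwise releasing it.
; AffectHealth handles death by disabling input, then after a delay requesting a game-mode respawn and destroying character and weapon.
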(event `self.ReceiveBeginPlay`
  (bind _mesh (`self.Mesh`))
  (`|ExecutionSequence`
    (:`then_0`
      ;[1 1 1] Attach Gun to Player Character at Runtime
      (bind _returnvalue (`|SpawnActorFromClass` "/Game/Blueprints/Weapon.Weapon_C" (`SceneComponent.K2_GetComponentToWorld` _mesh) "Undefined" "OverrideRootScale" null null))
      (bind _output_get (set `self.Weapon` _returnvalue))
      (`self.K2_AttachToComponent` _output_get _mesh "GunSocket" "SnapToTarget" "SnapToTarget" "KeepWorld" true))
    (:`then_1`
      ;[1 1 1] Set the Player Spawn Transform in the Game mode
      (bind _astwin_stick_mode (cast `/Game/Blueprints/TwinStickMode` (`GameplayStatics.GetGameMode`)))
      (bind _output_get_2 (set `self.GameMode` _astwin_stick_mode))
      (set `/Game/Blueprints/TwinStickMode.Player Spawn Transform` (`self.GetTransform`) _output_get_2))
    (:`then_2`
      ;[1 1 1] Set Up Score HUD
      (bind _returnvalue_2 (`|CreateWidget` "/Game/Blueprints/TwinStickHUD.TwinStickHUD_C"))
      (`UserWidget.AddToViewport` _returnvalue_2 0))))

(event `InputAxis|MoveUp`
  (params (AxisValue :type "Float (single-precision)"))
  ;[1 1 1] Movement
  (`self.AddMovementInput` (1.0 0.0 0.0) AxisValue))

(event `InputAxis|LookUp`
  (params (AxisValue :type "Float (single-precision)"))
  (bind _weapon (`self.Weapon`))
  ;[1 1 1] Set Player Rotation and Controls
  (bind _returnvalue (`KismetMathLibrary.MakeVector` AxisValue (stale `InputAxis|LookRight` AxisValue)))
  (if (> (`KismetMathLibrary.VSize` _returnvalue) 0.25) :!label _label
    (`Controller.SetControlRotation` (`self.GetController`) (`KismetMathLibrary.MakeRotFromX` _returnvalue))
    ;[1 1 1] Fire and Don't fire when time
    (`/Game/Blueprints/Weapon.PullTrigger` _weapon)
    (else
      (`/Game/Blueprints/Weapon.ReleaseTrigger` _weapon))))

(event `InputAxis|LookRight`
  (params (AxisValue :type "Float (single-precision)"))
  ;[1 1 1] Set Player Rotation and Controls
  (goto _label))

(event `InputAxis|MoveRight`
  (params (AxisValue :type "Float (single-precision)"))
  ;[1 1 1] Movement
  (`self.AddMovementInput` (0.0 1.0 0.0) AxisValue))

(event `/Game/Blueprints/iDamageable.AffectHealth`
  (params (Delta :type "Float (single-precision)"))
  ;[1 1 1] Destroy Player and Weapon when isDead = true. Delay before respawning
  (`self.CalculateHealth` Delta)
  (if (`self.isDead`)
    (`self.DisableInput` null)
    (`KismetSystemLibrary.Delay` 3.0)
    (`/Game/Blueprints/TwinStickMode.RespawnPlayer` (`self.GameMode`))
    (`self.K2_DestroyActor` (`self.Weapon`))
    (`self.K2_DestroyActor` self)))

(fn `UserConstructionScript`)