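; Weapon Blueprint that automatically fires single or twin projectiles while the trigger is held.
; PullTrigger passes a DoOnce gate to loop a timer at RoundsPerSecond, calling the event named in ProjectileFunction; ReleaseTrigger clears both fire timers and resets the gate.
; Fire and FireTwin clear each other's timer and spawn at ProjectileSpawnPoint.
; FireTwin offsets its pair along world X or Y, chosen from player 0's yaw quadrant.
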(event `PullTrigger`
  ;[1 1 1] Determine when to fire weapon
  (`/Engine/EditorBlueprintResources/StandardMacros.DoOnce` false :!label _label
    (:`Completed`
      (`KismetSystemLibrary.K2_SetTimer` null (`self.ProjectileFunction`) (/ 1.0 (`self.RoundsPerSecond`)) true))))

(event `ReleaseTrigger`
  ;[1 1 1] Determine when to fire weapon
  (`KismetSystemLibrary.K2_ClearTimer` null "Fire")
  (`KismetSystemLibrary.K2_ClearTimer` null "FireTwin")
  (goto _label :!via `Reset`))

(event `Fire`
  ;[1 1 1] Fire Green Projectile Event
  (`KismetSystemLibrary.K2_ClearTimer` null "FireTwin")
  (`|SpawnActorFromClass` "/Game/Blueprints/Projectile.Projectile_C" (`SceneComponent.K2_GetComponentToWorld` (`self.ProjectileSpawnPoint`)) "Undefined" "OverrideRootScale" null null))

(event `FireTwin`
  (bind (_returnvalue_roll _returnvalue_pitch _returnvalue_yaw) (`KismetMathLibrary.BreakRotator` (`self.K2_GetActorRotation` (`GameplayStatics.GetPlayerCharacter` 0))))
  (bind (_returnvalue_location _returnvalue_rotation _returnvalue_scale) (`KismetMathLibrary.BreakTransform` (`SceneComponent.K2_GetComponentToWorld` (`self.ProjectileSpawnPoint`))))
  (bind (_returnvalue_location_2 _returnvalue_rotation_2 _returnvalue_scale_2) (`KismetMathLibrary.BreakTransform` (`SceneComponent.K2_GetComponentToWorld` (`self.ProjectileSpawnPoint`))))
  ;[1 1 1] Fire Twin Bullet Upgrade
  (`KismetSystemLibrary.K2_ClearTimer` null "Fire")
  (if (or (and (>= _returnvalue_yaw -45.0) (< _returnvalue_yaw 46.0)) (and (>= _returnvalue_yaw 135.0) (< _returnvalue_yaw 226.0)) (and (>= _returnvalue_yaw -225.0) (< _returnvalue_yaw -135.0)))
    ;;[1 1 1] North South Bullet Modifiers
    (`|SpawnActorFromClass` "/Game/Blueprints/TwinProjectile.TwinProjectile_C" (`KismetMathLibrary.MakeTransform` (+ _returnvalue_location (0.0 -10.0 0.0)) _returnvalue_rotation _returnvalue_scale) "Undefined" "OverrideRootScale" null null)
    (`|SpawnActorFromClass` "/Game/Blueprints/TwinProjectile.TwinProjectile_C" (`KismetMathLibrary.MakeTransform` (+ _returnvalue_location (0.0 10.0 0.0)) _returnvalue_rotation _returnvalue_scale) "Undefined" "OverrideRootScale" null null)
    (else
      ;;[1 1 1] East West Bullet Modifiers
      (`|SpawnActorFromClass` "/Game/Blueprints/TwinProjectile.TwinProjectile_C" (`KismetMathLibrary.MakeTransform` (+ _returnvalue_location_2 (-10.0 0.0 0.0)) _returnvalue_rotation_2 _returnvalue_scale_2) "Undefined" "OverrideRootScale" null null)
      (`|SpawnActorFromClass` "/Game/Blueprints/TwinProjectile.TwinProjectile_C" (`KismetMathLibrary.MakeTransform` (+ _returnvalue_location_2 (10.0 0.0 0.0)) _returnvalue_rotation_2 _returnvalue_scale_2) "Undefined" "OverrideRootScale" null null))))

(fn `UserConstructionScript`)